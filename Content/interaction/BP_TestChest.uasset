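; Test chest that an interactor can open for a cost, spawning a BP_TestItem just above it.
; On interact press, it checks an attribute on the interactor's Ability System Component against the absolute Cost.
; If affordable, it applies GE_AddMoney to the interactor with the signed Cost as a SetByCaller magnitude, then disables further interaction and spawns the item.
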(event EventBeginPlay)

(event Collision|EventActorBeginOverlap
  (params (OtherActor :type Actor%20Object%20Reference)))

(event EventTick
  (params (DeltaSeconds :type Float%20%28single-precision%29)))

(event EventInteractPress
  (params (Interactor :type DR%20Base%20Character%20Object%20Reference))
  (bind _returnvalue (Ability|GetAbilitySystemComponent Interactor))
  (bind _cost (Variables|Default|GetCost))
  (bind (_bfound _returnvalue_2) (Class|AbilitySystemComponent|GetGameplayAttributeValue _returnvalue "(AttributeName=\"CurrentMoney\",Attribute=/Script/DeadRain.DRCharacterSet:CurrentMoney,AttributeOwner=\"/Script/CoreUObject.Class'/Script/DeadRain.DRCharacterSet'\")"))
  (if _bfound
    (if (>= _returnvalue_2 (Class|KismetMathLibrary|AbsInt64 _cost))
      (bind _returnvalue_3 (Ability|GameplayEffect|AssignTagSetbyCallerMagnitude (GameplayEffects|MakeOutgoingSpec :self _returnvalue :GameplayEffectClass "/Game/gas/GE_AddMoney.GE_AddMoney_C") "(TagName=\"Data.AddMoney\")" (Math|Conversions|ToFloat(Integer) _cost)))
      (GameplayEffects|ApplyGameplayEffectSpecToSelf _returnvalue _returnvalue_3)
      (Variables|Default|SetbIsInteractable false)
      (CallFunction|SpawnItem))))

(fn ConstructionScript)

(fn SpawnItem
  (Game|SpawnActorfromClass "/Game/interaction/BP_TestItem.BP_TestItem_C" (Math|Transform|MakeTransform (+ (Transformation|GetActorLocation) "0.000000,0.000000,50.000000") "0, 0, 0" "1.000000,1.000000,1.000000") "AlwaysSpawn" "MultiplyWithRoot" 0 0))