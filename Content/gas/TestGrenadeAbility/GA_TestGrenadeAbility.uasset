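; GA_TestGrenadeAbility is a test Gameplay Ability that spawns a grenade actor in front of the avatar.
; After committing and casting the avatar to Pawn, it spawns GrenadeActorClass slightly ahead along the forward vector, with the avatar as Owner and Instigator.
; The ability ends right after spawning, but a failed commit or cast exits without calling EndAbility.
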(event Ability|EventActivateAbility
  (bind _returnvalue (Ability|GetAvatarActorfromActorInfo))
  (bind _returnvalue_2 (Transformation|GetActorTransform _returnvalue))
  (bind _returnvalue_3 (Ability|CommitAbility))
  (if _returnvalue_3
    (bind _aspawn (Utilities|Casting|CastToPawn _returnvalue))
    (Game|SpawnActorfromClass (Variables|Default|GetGrenadeActorClass) (Math|Transform|MakeTransform (+ (.location _returnvalue_2) (* (Transformation|GetActorForwardVector _returnvalue) 5e+01)) (.rotation _returnvalue_2) (.scale _returnvalue_2)) "AdjustIfPossibleButAlwaysSpawn" "MultiplyWithRoot" _returnvalue _aspawn)
    (Ability|EndAbility)))

(event Ability|EventOnEndAbility
  (params (bWasCancelled :type Boolean)))