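; Timed grenade projectile actor, apparently for a test gameplay ability, that deals area damage to characters.
; BeginPlay sets the projectile speed and starts a fuse timer that calls Explode.
; Explode spawns an attached particle effect, sphere-overlaps for DRBaseCharacter actors and has the owning character apply the GAS test damage effect to each.
; DestroyActor sits inside the hit loop and also runs when nothing overlaps.
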(event EventBeginPlay
  (Variables|/Script/Engine.ProjectileMovementComponent|SetInitialSpeed (Variables|Default|GetProjectileMovement) 1e+03)
  (Utilities|Time|SetTimerbyFunctionName 0 "Explode" (Math|Float|MakeLiteralFloat 3.0)))

(event Collision|EventActorBeginOverlap
  (params (OtherActor :type Actor%20Object%20Reference)))

(event EventTick
  (params (DeltaSeconds :type Float%20%28single-precision%29)))

(fn ConstructionScript)

(fn Explode
  (Effects|SpawnEmitterAttached "/Engine/Tutorial/SubEditors/TutorialAssets/TutorialParticleSystem.TutorialParticleSystem" (Variables|Default|GetSphere) "None" "0, 0, 0" "0, 0, 0" "1.000000,1.000000,1.000000" "SnapToTargetIncludingScale")
  (bind (_outactors _returnvalue) (Collision|SphereOverlapActors (Transformation|GetActorLocation) 3e+02 (LocalVariables|GetNewLocalVar_0) "/Script/DeadRain.DRBaseCharacter"))
  (if _returnvalue
    (bind _asdrbase_character (Utilities|Casting|CastToDRBaseCharacter (Components|GetOwner)))
    (for _array_element _outactors
      (bind _asdrbase_character_2 (Utilities|Casting|CastToDRBaseCharacter _array_element))
      (Class|DRBaseCharacter|ApplyGameplayEffecttoTarget _asdrbase_character "/Game/weapon/Gun/GE_TestDamageEffect.GE_TestDamageEffect_C" _asdrbase_character_2)
      (Actor|DestroyActor))
    (else
      (Actor|DestroyActor))))