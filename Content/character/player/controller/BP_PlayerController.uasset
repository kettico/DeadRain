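; Player controller that adds the main Enhanced Input mapping context and routes input to the controlled pawn.
; Move feeds the character's movement component along pawn forward and right vectors, and look adds yaw and inverted pitch.
; Interact press and hold call the player character's current interactable, while three weapon inputs trigger its weapon actions.
; Ability 1 activates a test grenade Gameplay Ability by class through the character's AbilitySystemComponent.
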(event EventBeginPlay
  (bind _returnvalue (PlayerController|LocalPlayerSubsystems|GetEnhancedInputLocalPlayerSubsystem))
  (Utilities|IsValid _returnvalue
    (:Is%20Valid
      (Input|AddMappingContext _returnvalue "/Game/character/player/controller/IMC_Main/IMC_Main.IMC_Main" 0 "(bIgnoreAllPressedKeysUntilRelease=True,bForceImmediately=False,bNotifyUserSettings=False)"))))

(event Input|EnhancedActionEvents|EnhancedInputActionIA_Move
  (params (ActionValue :type Vector%202D%20Structure) (ElapsedSeconds :type Float%20%28double-precision%29) (TriggeredSeconds :type Float%20%28double-precision%29) (InputAction :type Input%20Action%20Object%20Reference :default "/Game/character/player/controller/IMC_Main/IA_Move.IA_Move"))
  (bind _returnvalue (Pawn|GetControlledPawn))
  (bind _returnvalue_2 (Pawn|GetControlledPawn))
  (Utilities|IsValid _returnvalue
    (:Is%20Valid
      (bind _ascharacter (Utilities|Casting|CastToCharacter _returnvalue))
      (Class|PawnMovementComponent|AddInputVector (Variables|/Script/Engine.Character|GetCharacterMovement _ascharacter) (+ (* (.x ActionValue) (Transformation|GetActorForwardVector _returnvalue_2)) (* (Transformation|GetActorRightVector _returnvalue_2) (.y ActionValue))) false))))

(event Input|EnhancedActionEvents|EnhancedInputActionIA_Look
  (params (ActionValue :type Vector%202D%20Structure) (ElapsedSeconds :type Float%20%28double-precision%29) (TriggeredSeconds :type Float%20%28double-precision%29) (InputAction :type Input%20Action%20Object%20Reference :default "/Game/character/player/controller/IMC_Main/IA_Look.IA_Look"))
  (bind _returnvalue (Pawn|GetControlledPawn))
  (Utilities|IsValid _returnvalue
    (:Is%20Valid
      (Pawn|Input|AddControllerYawInput _returnvalue (.x ActionValue))
      (Pawn|Input|AddControllerPitchInput _returnvalue (- 0.0 (.y ActionValue))))))

(event Input|EnhancedActionEvents|EnhancedInputActionIA_InteractHold
  (params (ActionValue :type Boolean) (ElapsedSeconds :type Float%20%28double-precision%29) (TriggeredSeconds :type Float%20%28double-precision%29) (InputAction :type Input%20Action%20Object%20Reference :default "/Game/character/player/controller/IMC_Main/IA_InteractHold.IA_InteractHold"))
  (bind _returnvalue (Pawn|GetControlledPawn))
  (Utilities|IsValid _returnvalue
    (:Is%20Valid
      (bind _asbp_player_character (Utilities|Casting|CastToBP_PlayerCharacter _returnvalue))
      (Utilities|IsValid (Class|DRPlayerCharacter|GetCurrentInteractable _asbp_player_character)
        (:Is%20Valid
          (Class|DRInteractableActor|InteractHold (Class|DRPlayerCharacter|GetCurrentInteractable _asbp_player_character) _asbp_player_character))))))

(event Input|EnhancedActionEvents|EnhancedInputActionIA_InteractPress
  (params (ActionValue :type Boolean) (ElapsedSeconds :type Float%20%28double-precision%29) (TriggeredSeconds :type Float%20%28double-precision%29) (InputAction :type Input%20Action%20Object%20Reference :default "/Game/character/player/controller/IMC_Main/IA_InteractPress.IA_InteractPress"))
  (bind _returnvalue (Pawn|GetControlledPawn))
  (Utilities|IsValid _returnvalue
    (:Is%20Valid
      (bind _asbp_player_character (Utilities|Casting|CastToBP_PlayerCharacter _returnvalue))
      (Utilities|IsValid (Class|DRPlayerCharacter|GetCurrentInteractable _asbp_player_character)
        (:Is%20Valid
          (Class|DRInteractionInterface|InteractPress (Class|DRPlayerCharacter|GetCurrentInteractable _asbp_player_character) _asbp_player_character)
          (Development|PrintString (Utilities|String|Append "Interact with : " (Utilities|GetDisplayName (Class|DRPlayerCharacter|GetCurrentInteractable _asbp_player_character)))))))))

(event Input|EnhancedActionEvents|EnhancedInputActionIA_Primary
  (params (ActionValue :type Boolean) (ElapsedSeconds :type Float%20%28double-precision%29) (TriggeredSeconds :type Float%20%28double-precision%29) (InputAction :type Input%20Action%20Object%20Reference :default "/Game/character/player/controller/IMC_Main/IA_Primary.IA_Primary"))
  (bind _asbp_player_character (Utilities|GetBPPlayerCharacter))
  (Class|DRBaseCharacter|ActivateWeaponPrimary _asbp_player_character))

(event Input|EnhancedActionEvents|EnhancedInputActionIA_Secondary
  (params (ActionValue :type Boolean) (ElapsedSeconds :type Float%20%28double-precision%29) (TriggeredSeconds :type Float%20%28double-precision%29) (InputAction :type Input%20Action%20Object%20Reference :default "/Game/character/player/controller/IMC_Main/IA_Secondary.IA_Secondary"))
  (bind _asbp_player_character (Utilities|GetBPPlayerCharacter))
  (Class|DRBaseCharacter|ActivateWeaponSecondary _asbp_player_character))

(event Input|EnhancedActionEvents|EnhancedInputActionIA_Tertiary
  (params (ActionValue :type Boolean) (ElapsedSeconds :type Float%20%28double-precision%29) (TriggeredSeconds :type Float%20%28double-precision%29) (InputAction :type Input%20Action%20Object%20Reference :default "/Game/character/player/controller/IMC_Main/IA_Tertiary.IA_Tertiary"))
  (bind _asbp_player_character (Utilities|GetBPPlayerCharacter))
  (Class|DRBaseCharacter|ActivateWeaponTertiary _asbp_player_character))

(event Input|EnhancedActionEvents|EnhancedInputActionIA_Ability1
  (params (ActionValue :type Boolean) (ElapsedSeconds :type Float%20%28double-precision%29) (TriggeredSeconds :type Float%20%28double-precision%29) (InputAction :type Input%20Action%20Object%20Reference :default "/Game/character/player/controller/IMC_Main/IA_Ability1.IA_Ability1"))
  (Development|PrintString "START: ABILITY 1")
  (bind _asbp_player_character (Utilities|GetBPPlayerCharacter))
  (bind _abilitysystemcomponent (Variables|/Script/DeadRain.DRBaseCharacter|GetAbilitySystemComponent _asbp_player_character)
    (:then
      (Abilities|TryActivateAbilitybyClass _abilitysystemcomponent "/Game/gas/TestGrenadeAbility/GA_TestGrenadeAbility.GA_TestGrenadeAbility_C" true))
    (:else)))

(fn ConstructionScript)